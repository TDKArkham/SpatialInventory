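; Player controller for the inventory system that toggles the inventory screen on the ToggleInventory input action.
; When opening, it creates a WBP_Inventory bound to the controlled pawn's inventory component, adds it to the viewport, focuses it and shows the cursor.
; When closing, it removes and clears the widget, then restores game-only input and hides the cursor.
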(event Input|ActionEvents|InputActionToggleInventory
  (params (Key :type Key%20Structure :default "None"))
  (bind _self self)
  (bind _self_2 self)
  (:Pressed
    (Variables|Default|GetInventoryWidget
      (:then
        (Widget|RemovefromParent (Variables|Default|GetInventoryWidget))
        (Variables|Default|SetInventoryWidget 0)
        (Input|SetInputModeGameOnly _self_2)
        (Variables|/Script/Engine.PlayerController|SetbShowMouseCursor _self_2 false))
      (:else
        (bind _returnvalue (UserInterface|CreateWidget "/Game/InventorySystem/UI/WBP_Inventory.WBP_Inventory_C" 0 (Class|InventoryComponent|GetInventoryComponent (Pawn|GetControlledPawn)) 5e+01))
        (bind _output_get (Variables|Default|SetInventoryWidget _returnvalue))
        (UserInterface|Viewport|AddtoViewport _output_get 0)
        (Input|SetInputModeGameandUI _self _output_get "DoNotLock" false)
        (Variables|/Script/Engine.PlayerController|SetbShowMouseCursor _self true)))))

(fn ConstructionScript)